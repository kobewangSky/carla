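; CARLA pedestrian Blueprint that randomizes a walker's look and reacts to weather and vehicle hits.
; Construction rolls a weighted skin tone and, via SetProps, a socket-attached umbrella in rain or a random prop otherwise, usually setting walk speed too.
; Weather changes destroy and reroll the held item.
; Body or prop trigger overlaps with a vehicle's skeletal mesh apply damage, enable ragdoll and prop physics, then destroy the walker after a delay.
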(event OnComponentBeginOverlap(CapsuleComponent)
  (params (OverlappedComponent :type Primitive%20Component%20Object%20Reference) (OtherActor :type Actor%20Object%20Reference) (OtherComp :type Primitive%20Component%20Object%20Reference) (OtherBodyIndex :type Integer) (bFromSweep :type Boolean) (SweepResult :type Hit%20Result%20Structure%20%28by%20ref%29))
  ;[1 1 1] speed Up crossing the road
  (Utilities|Casting|CastToRoadNavigationClass "/Game/Blueprints/RoadNavigation.RoadNavigation_C")
  (bind _ascharacter_movement_component (Utilities|Casting|CastToCharacterMovementComponent (Variables|Character|GetCharacterMovement))))

(event OnComponentEndOverlap(CapsuleComponent)
  (params (OverlappedComponent :type Primitive%20Component%20Object%20Reference) (OtherActor :type Actor%20Object%20Reference) (OtherComp :type Primitive%20Component%20Object%20Reference) (OtherBodyIndex :type Integer))
  ;[1 1 1] speed Up crossing the road
  (Utilities|Casting|CastToRoadNavigationClass "/Game/Blueprints/RoadNavigation.RoadNavigation_C")
  (bind _ascharacter_movement_component (Utilities|Casting|CastToCharacterMovementComponent (Variables|Character|GetCharacterMovement))))

(event OnComponentBeginOverlap(PedestrianDeathTrigger)
  (params (OverlappedComponent :type Primitive%20Component%20Object%20Reference) (OtherActor :type Actor%20Object%20Reference) (OtherComp :type Primitive%20Component%20Object%20Reference) (OtherBodyIndex :type Integer) (bFromSweep :type Boolean) (SweepResult :type Hit%20Result%20Structure%20%28by%20ref%29))
  (Utilities|HitbySomething OtherActor OtherComp))

(event OnComponentBeginOverlap(PedestrianPropDeathTrigger)
  (params (OverlappedComponent :type Primitive%20Component%20Object%20Reference) (OtherActor :type Actor%20Object%20Reference) (OtherComp :type Primitive%20Component%20Object%20Reference) (OtherBodyIndex :type Integer) (bFromSweep :type Boolean) (SweepResult :type Hit%20Result%20Structure%20%28by%20ref%29))
  (Utilities|HitbySomething OtherActor OtherComp))

(event Custom|NotifyChangeOfWeather
  (params (ItIsRaining :type Boolean))
  (bind _holdmesh (Variables|Components|GetHoldMesh))
  (bind _returnvalue (Utilities|IsValid _holdmesh))
  ;[1 1 1] Destroy Umbrella/Prop Whenchanging climate
  (if ItIsRaining
    (if _returnvalue
      (Components|DestroyComponent _holdmesh))
    (CallFunction|Rain false)
    (else
      (if _returnvalue
        (Components|DestroyComponent _holdmesh))
      (bind _returnvalue_2 (Class|RandomEngine|GetNormalDistribution (Variables|Random|GetRandomEngine) 1.2e+02 5e+01))
      (CallFunction|SetProps))))

(event Collision|EventActorBeginOverlap
  (params (OtherActor :type Actor%20Object%20Reference)))

(fn ConstructionScript
  (CallFunction|SetProps)
  (CallFunction|SkinTone))

(fn SetProps
  (bind _randomengine (Variables|Random|GetRandomEngine))
  (bind _ascarla_game_instance (Utilities|Casting|CastToCarlaGameInstance (Game|GetGameInstance)))
  (bind _returnvalue (Class|CarlaGameInstance|GetCARLASettings _ascarla_game_instance))
  (|CollapseGraph_0 _returnvalue
    (:Raining
      (CallFunction|Rain false))
    (:NotRaining
      (bind _returnvalue_2 (Class|RandomEngine|GetBoolwithWeight _randomengine 5e+01))
      (if _returnvalue_2
        (bind _returnvalue_3 (Class|RandomEngine|GetIntwithWeight _randomengine (Variables|Default|GetItemChances2)))
        (CallFunction|Prop (.Prop (Utilities|Struct|BreakWalkerprops (Utilities|Array|Get(acopy) (Variables|Default|GetWalkerProps) _returnvalue_3))) (.SocketName (Utilities|Struct|BreakWalkerprops (Utilities|Array|Get(acopy) (Variables|Default|GetWalkerProps) _returnvalue_3))) (.MinSpeed (Utilities|Struct|BreakWalkerprops (Utilities|Array|Get(acopy) (Variables|Default|GetWalkerProps) _returnvalue_3))) (.MaxSpeed (Utilities|Struct|BreakWalkerprops (Utilities|Array|Get(acopy) (Variables|Default|GetWalkerProps) _returnvalue_3))) (.RelativeTransform (Utilities|Struct|BreakWalkerprops (Utilities|Array|Get(acopy) (Variables|Default|GetWalkerProps) _returnvalue_3)))) ; BriefCase
        (Variables|Default|Setanimation (.Anim (Utilities|Struct|BreakWalkerprops (Utilities|Array|Get(acopy) (Variables|Default|GetWalkerProps) _returnvalue_3))))))))

(fn Prop
  (params (Prop%20to%20place :type Static%20Mesh%20Object%20Reference) (SocketName :type Name) (WalkSpeedMin :type Float%20%28single-precision%29) (WalkSpeedMax :type Float%20%28single-precision%29) (RelativeTransform :type Transform))
  (bind _returnvalue (StaticMesh|GetBoundingBox Prop%20to%20place))
  (bind _pedestrianpropdeathtrigger (Variables|Components|GetPedestrianPropDeathTrigger))
  (bind _returnvalue_2 (- (.z (.max _returnvalue)) (.z (.min _returnvalue))))
  (bind _returnvalue_3 (/ _returnvalue_2 2.0))
  (Utilities|FlowControl|Sequence
    (:then_0
      (bind _returnvalue_4 (AddComponent|AddStaticMeshComponent false RelativeTransform))
      (Variables|Components|SetHoldMesh _returnvalue_4)
      (Components|StaticMesh|SetStaticMesh (Variables|Components|GetHoldMesh) Prop%20to%20place)
      (Transformation|AttachComponentToComponent (Variables|Components|GetHoldMesh) (Variables|Character|GetMesh) SocketName "KeepRelative" "KeepRelative" "KeepRelative" true)
      (Collision|SetCollisionEnabled (Variables|Components|GetHoldMesh) "NoCollision")
      (bind _ascarla_game_instance (Utilities|Casting|CastToCarlaGameInstance (Game|GetGameInstance)))
      (Class|CarlaGameInstance|GetCARLASettings _ascarla_game_instance)
      (Class|PrimitiveComponent|SetCullDistance _returnvalue_4 0.0))
    (:then_1
      (Transformation|AttachComponentToComponent _pedestrianpropdeathtrigger (Variables|Components|GetHoldMesh) "None" "KeepRelative" "KeepRelative" "KeepRelative" true)
      (Components|Box|SetBoxExtent _pedestrianpropdeathtrigger (Math|Vector|MakeVector (+ (/ (- (.x (.max _returnvalue)) (.x (.min _returnvalue))) 2.0) 1e+01) (+ (/ (- (.y (.max _returnvalue)) (.y (.min _returnvalue))) 2.0) 1e+01) (+ _returnvalue_3 1e+01)) true)
      (Transformation|SetRelativeTransform _pedestrianpropdeathtrigger (Math|Transform|MakeTransform (Math|Vector|MakeVector 0.0 0.0 (- 1.0 _returnvalue_3)) "0, 0, 0" "1,1,1") true false))
    (:then_2
      (bind _returnvalue_5 (Class|RandomEngine|GetUniformFloatinRange (Variables|Random|GetRandomEngine) WalkSpeedMin WalkSpeedMax))
      (Variables|/Script/Engine.CharacterMovementComponent|SetMaxWalkSpeed (Variables|Character|GetCharacterMovement) _returnvalue_5))
    (:then_3
      (return (Variables|Character|GetMesh) Prop%20to%20place (Variables|Components|GetHoldMesh)))))

(fn Default
  (params (Animations :type Array%20of%20Object%20Class%20References))
  (if (Variables|Default|GetUsesDefault)
    (bind _returnvalue (Class|RandomEngine|GetUniformIntinRange (Variables|Random|GetRandomEngine) 0 (- (Utilities|Array|Length Animations) 1)))
    (Components|SkeletalMesh|SetAnimInstanceClass (Variables|Character|GetMesh) (Utilities|Array|Get(acopy) Animations _returnvalue))))

(fn Rain
  (params (Condition :type Boolean))
  (if (> 9 (Math|Random|RandomIntegerinRange 0 10))
    (Variables|Default|SetHoldsUmbrella true)
    (bind _propcomponent_ (CallFunction|Prop "/Game/Static/Pedestrians/Animations/PropRelated/UmbrellaWalk/Umbrella.Umbrella" "LeftHandGrabber" 5e+01 8e+01)) ; Umbrella
    (Variables|Components|SetHoldMesh _propcomponent_)
    (if (Utilities|IsValid _propcomponent_)
      (if (Utilities|Array|ContainsItem (Class|MeshComponent|GetMaterialSlotNames _propcomponent_) "Umbrella")
        (bind _returnvalue (Rendering|Material|CreateDynamicMaterialInstance _propcomponent_ (Utilities|Array|FindItem (Class|MeshComponent|GetMaterialSlotNames _propcomponent_) "Umbrella") "/Game/Static/Pedestrians/Animations/PropRelated/UmbrellaWalk/Umbrella_Mat.Umbrella_Mat" :!class /Script/Engine.PrimitiveComponent))
        (bind _returnvalue_2 (Class|RandomEngine|GetIntwithWeight (Variables|Random|GetRandomEngine) (Variables|Default|GetUmbrellaColorChances)))
        (Rendering|Material|SetVectorParameterValue _returnvalue "UmbrellaColor" (Utilities|Array|Get(acopy) (Variables|Default|GetUmbrellaColors) _returnvalue_2) :!class /Script/Engine.MaterialInstanceDynamic)
        (else
          (Development|PrintString "No material")))
      (else
        (Development|PrintString "no prop")))
    (else
      (Variables|/Script/Engine.CharacterMovementComponent|SetMaxWalkSpeed (Variables|Character|GetCharacterMovement) (Math|Random|RandomFloatinRange 2.5e+02 4e+02)))))

(fn BiasedRandom
  (params (Range :type Array%20of%20Floats%20%28single-precision%29))
  (LocalVariables|SetCurrentIndex (Utilities|Array|Length Range))
  (bind (_array_element _array_index) (Utilities|Array|ForEachLoopwithBreak Range :!label _label)
    (:LoopBody
      (if (< (Math|Random|RandomFloatinRange 0.0 (Utilities|Array|Get(acopy) Range (- (Utilities|Array|Length Range) 1))) _array_element)
        (LocalVariables|SetCurrentIndex _array_index)
        (goto _label Break)))
    (:Completed
      (return (LocalVariables|GetCurrentIndex)))))

(fn HitbyCar
  (bind _mesh (Variables|Character|GetMesh))
  (bind _holdmesh (Variables|Components|GetHoldMesh))
  (Game|Damage|ApplyDamage self 1.0 0 0 "/Script/Engine.DamageType")
  (if (Utilities|IsValid _holdmesh)
    (Transformation|DetachFromComponent _holdmesh "KeepWorld" "KeepWorld" "KeepWorld" true)
    (Physics|SetSimulatePhysics _holdmesh true)
    (Collision|SetCollisionEnabled _holdmesh "QueryAndPhysics"))
  (Physics|SetSimulatePhysics _mesh true)
  (Collision|SetCollisionEnabled _mesh "QueryAndPhysics")
  (Components|Box|SetBoxExtent (Variables|Components|GetPedestrianDeathTrigger) "1.000000,1.000000,1.000000" true)
  (Components|Box|SetBoxExtent (Variables|Components|GetPedestrianPropDeathTrigger) "1.000000,1.000000,1.000000" true)
  (Components|Box|SetBoxExtent (Variables|Components|GetCarStopper) "20.000000,20.000000,20.000000" true)
  (Components|Capsule|SetCapsuleSize (Variables|Collision|GetCapsuleComponent) 0.0 0.0 true)
  (Collision|SetCollisionResponsetoAllChannels (Variables|Character|GetMesh) "ECR_Block"))

(fn MaterialChange
  (params (TargetArray :type Array%20of%20Material%20Instance%20Object%20References) (MaterialSlotName :type Name) (Target :type Primitive%20Component%20Object%20Reference))
  (bind _returnvalue (Utilities|Array|Length TargetArray))
  (if (> _returnvalue 0)
    (bind _returnvalue_2 (Class|RandomEngine|GetUniformIntinRange (Variables|Random|GetRandomEngine) 0 (- _returnvalue 1)))
    (Rendering|Material|SetMaterialbyName Target MaterialSlotName (Utilities|Array|Get(acopy) TargetArray _returnvalue_2)))
  (return))

(fn MaterialStandar
  (params (Bottom :type Array%20of%20Material%20Instance%20Object%20References) (Tops :type Array%20of%20Material%20Instance%20Object%20References) (Footwear :type Array%20of%20Material%20Instance%20Object%20References) (Skin :type Array%20of%20Material%20Instance%20Object%20References) (ExtraMaterialArray :type Array%20of%20Material%20Instance%20Object%20References) (ExtraMaterialSlotName :type Name) (Target :type Primitive%20Component%20Object%20Reference))
  (bind _returnvalue (Class|RandomEngine|GetBoolwithWeight (Variables|Random|GetRandomEngine) 0.1))
  (if _returnvalue
    _
    (else
      (CallFunction|MaterialChange Bottom "bottom" Target)
      (CallFunction|MaterialChange Tops "top" Target)
      (CallFunction|MaterialChange Footwear "shoes" Target)
      (CallFunction|MaterialChange Skin "Skin" Target)
      (CallFunction|MaterialChange ExtraMaterialArray ExtraMaterialSlotName Target)))
  (return))

(fn CLothing
  (params (Materials :type Array%20of%20Texture%20Structs%20Structures) (ElementIndex :type Integer) (Value :type Array%20of%20Linear%20Color%20Structures) (Mesh :type Mesh%20Component%20Object%20Reference))
  (bind _randomengine (Variables|Random|GetRandomEngine))
  (bind _returnvalue (Class|RandomEngine|GetUniformIntinRange _randomengine 0 (- (Utilities|Array|Length Materials) 1)))
  (bind _returnvalue_2 (Class|RandomEngine|GetUniformIntinRange _randomengine 0 (- (Utilities|Array|Length Value) 1)))
  (bind _returnvalue_3 (Rendering|Material|CreateDynamicMaterialInstance Mesh ElementIndex (Utilities|Array|Get(acopy) (Rendering|Material|GetMaterials Mesh) ElementIndex) :!class /Script/Engine.PrimitiveComponent))
  (Rendering|Material|SetTextureParameterValue _returnvalue_3 "TiledTextureBaseColor" (.basecolor (Utilities|Array|Get(acopy) Materials _returnvalue)))
  (Rendering|Material|SetTextureParameterValue _returnvalue_3 "TiledTextureNormal" (.normal (Utilities|Array|Get(acopy) Materials _returnvalue)))
  (Rendering|Material|SetTextureParameterValue _returnvalue_3 "TiledTextureOclussionRoughnessMetallic" (.oclussionroughnessmetallic (Utilities|Array|Get(acopy) Materials _returnvalue)))
  (Rendering|Material|SetScalarParameterValue _returnvalue_3 "BasicTextureTiling" (.tiling (Utilities|Array|Get(acopy) Materials _returnvalue)) :!class /Script/Engine.MaterialInstanceDynamic)
  (Rendering|Material|SetVectorParameterValue _returnvalue_3 "Color" (Utilities|Array|Get(acopy) Value _returnvalue_2) :!class /Script/Engine.MaterialInstanceDynamic)
  (return _returnvalue_3))

(fn SkinTone
  (bind _mesh (Variables|Character|GetMesh))
  (if (and (Utilities|IsValid _mesh) (Class|MeshComponent|IsMaterialSlotNameValid _mesh "Skin"))
    (bind _returnvalue (Rendering|Material|CreateDynamicMaterialInstance "/Game/Static/Pedestrians/Materials/SkinMaterial.SkinMaterial" :!class /Script/Engine.KismetMaterialLibrary))
    (Rendering|Material|SetMaterial _mesh (Rendering|Material|GetMaterialIndex _mesh "Skin") _returnvalue)
    (bind _returnvalue_2 (Class|RandomEngine|GetIntwithWeight (Variables|Random|GetRandomEngine) (Variables|Default|GetSkinWeights)))
    (Rendering|Material|SetVectorParameterValueonMaterials _mesh "SkinTone" (Math|Conversions|ToVector(LinearColor) (Utilities|Array|Get(acopy) (Variables|Default|GetSkinTones) _returnvalue_2)))))