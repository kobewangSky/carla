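; Weather controller actor that sets the sky look, ground wetness and rain for a level from its own variables.
; Its construction script overrides the first BP_Sky_Sphere's colors, clouds and sun, and writes water limits to the WetRoadComplexParam material parameter collection.
; BeginPlay attaches GPU rain particles to the player pawn.
; Directional light, skylight and post-process helpers exist but are not run; RefreshWeather is empty.
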(event EventBeginPlay
  (CallFunction|RainParticles))

(event Collision|EventActorBeginOverlap
  (params (OtherActor :type Actor%20Object%20Reference)))

(event EventTick
  (params (DeltaSeconds :type Float%20%28single-precision%29)))

(fn ConstructionScript
  (CallFunction|SkySphere)
  (CallFunction|RainGround))

(fn SkyLight
  (bind _outactors (Actor|GetAllActorsOfClass "/Script/Engine.SkyLight"))
  (Rendering|Components|Light|SetIntensity (Variables|/Script/Engine.SkyLight|GetLightComponent (Utilities|Array|Get(acopy) _outactors)) (Variables|Default|GetSkyLightIntensity))
  (Rendering|Components|Light|SetLightColor (Variables|/Script/Engine.SkyLight|GetLightComponent (Utilities|Array|Get(acopy) _outactors)) (Variables|Default|GetSkyLightColor))
  (Class|SkyLightComponent|SetIndirectLightingIntensity (Variables|/Script/Engine.SkyLight|GetLightComponent (Utilities|Array|Get(acopy) _outactors)) (Variables|Default|GetIndirectLightIntensity)))

(fn DirectionalLight
  (bind _outactors (Actor|GetAllActorsOfClass "/Script/Engine.DirectionalLight"))
  (Transformation|SetActorRotation (Utilities|Array|Get(acopy) _outactors) (Variables|Default|GetSunDirection))
  (Rendering|Components|Light|SetIntensity (Variables|/Script/Engine.Light|GetLightComponent (Utilities|Array|Get(acopy) _outactors)) (Variables|Default|GetDirectionalLightIntensity))
  (Rendering|Components|Light|SetLightColor (Variables|/Script/Engine.Light|GetLightComponent (Utilities|Array|Get(acopy) _outactors)) (Variables|Default|GetDirectionalLightColor) true)
  (Class|LightComponent|SetIndirectLightingIntensity (Variables|/Script/Engine.Light|GetLightComponent (Utilities|Array|Get(acopy) _outactors)) (Variables|Default|GetIndirectLightingIIntensity))
  (Class|LightComponent|SetEnableLightShaftBloom (Variables|/Script/Engine.Light|GetLightComponent (Utilities|Array|Get(acopy) _outactors)) (Variables|Default|GetBloom)))

(fn SkySphere
  (bind _outactors (Actor|GetAllActorsOfClass "/Engine/EngineSky/BP_Sky_Sphere.BP_Sky_Sphere_C"))
  (Variables|/Engine/EngineSky/BP_Sky_Sphere.BP_Sky_Sphere_C|SetColors%20determined%20by%20sun%20position (Utilities|Array|Get(acopy) _outactors) false)
  (Variables|/Engine/EngineSky/BP_Sky_Sphere.BP_Sky_Sphere_C|SetSun%20brightness (Utilities|Array|Get(acopy) _outactors) (Variables|Default|GetSunBrightness))
  (Variables|/Engine/EngineSky/BP_Sky_Sphere.BP_Sky_Sphere_C|SetCloud%20opacity (Utilities|Array|Get(acopy) _outactors) (Variables|Default|GetCloudOpacity))
  (Variables|/Engine/EngineSky/BP_Sky_Sphere.BP_Sky_Sphere_C|SetSun%20height (Utilities|Array|Get(acopy) _outactors) (Variables|Default|GetSunHeight))
  (Variables|/Engine/EngineSky/BP_Sky_Sphere.BP_Sky_Sphere_C|SetHorizon%20Falloff (Utilities|Array|Get(acopy) _outactors) (Variables|Default|GetHorizontFalloff))
  (Variables|/Engine/EngineSky/BP_Sky_Sphere.BP_Sky_Sphere_C|SetZenith%20Color (Utilities|Array|Get(acopy) _outactors) (Variables|Default|GetZenithColor))
  (Variables|/Engine/EngineSky/BP_Sky_Sphere.BP_Sky_Sphere_C|SetHorizon%20color (Utilities|Array|Get(acopy) _outactors) (Variables|Default|GetHorizonColor))
  (Variables|/Engine/EngineSky/BP_Sky_Sphere.BP_Sky_Sphere_C|SetCloud%20color (Utilities|Array|Get(acopy) _outactors) (Variables|Default|GetCloudColor))
  (Variables|/Engine/EngineSky/BP_Sky_Sphere.BP_Sky_Sphere_C|SetOverall%20Color (Utilities|Array|Get(acopy) _outactors) (Variables|Default|GetOverallColor)))

(fn RainGround
  (Rendering|Material|SetScalarParameterValue "/Game/Static/GenericMaterials/WetPavement/WetRoadComplexParam.WetRoadComplexParam" "Min water" (Variables|Default|GetMinWater) :!class /Script/Engine.KismetMaterialLibrary)
  (Rendering|Material|SetScalarParameterValue "/Game/Static/GenericMaterials/WetPavement/WetRoadComplexParam.WetRoadComplexParam" "Max water" (Variables|Default|GetMaxWater) :!class /Script/Engine.KismetMaterialLibrary))

(fn RainParticles
  (bind _returnvalue (AddComponent|AddParticleSystemComponent (Game|Player|GetPlayerPawn 0) false))
  (Effects|SpawnEmitterAttached "/Game/Static/GenericMaterials/rain/P_GPU_particles_collision2.P_GPU_particles_collision2" _returnvalue "None" (Variables|Default|GetRainPlacement)))

(fn NewFunction0
  (bind _outactors (Actor|GetAllActorsOfClass "/Script/Engine.PostProcessVolume"))
  (Variables|/Script/Engine.PostProcessVolume|SetSettings (Utilities|Array|Get(acopy) _outactors) (Utilities|Struct|MakePostProcessSettings 888.0 888.0)))

(fn RefreshWeather
  (params (NewParam :type Vector)))