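; CARLA weather actor that applies the current weather description to the level, with an input action to cycle through weather presets at runtime.
; On refresh it updates the sun light, skylight, sky sphere material and rain particles, and switches artificial lights on when the sun angle indicates night.
; A material parameter collection drives road wetness and ripples, and a spring arm attaches to the player pawn at BeginPlay.
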(event EventRefreshWeather
  (CallFunction|UpdateEnvironmentActors))

(event EventBeginPlay
  (Transformation|AttachComponentToComponent (Variables|Default|GetSpringArm) (VehicleSound|GetRootComponent (Game|Player|GetPlayerPawn 0)) "None" "KeepRelative" "KeepRelative" "KeepRelative" true))

(event Input|ActionEvents|InputActionChangeWeather
  (params (Key :type Key%20Structure))
  (:Pressed
    (bind _israining (CallFunction|ChangeWeatheratRuntime))))

(fn ConstructionScript)

(fn UpdateEnvironmentActors
  (CallFunction|UpdateDirectionalLight)
  (CallFunction|SetSkylight)
  (CallFunction|SetNightDay)
  (CallFunction|SetPrecipitations)
  (CallFunction|SetArtificialLighting)
  (CallFunction|UpdateSky))

(fn UpdateSky
  (bind _returnvalue (Class|DynamicWeather|GetWeatherDescription))
  (bind (_name _sunpolarangle _sunbrightness _cloudopacity _horizontfalloff _zenithcolor _horizoncolor _cloudcolor _overallskycolor) (Utilities|Struct|BreakWeatherDescription _returnvalue))
  (bind (_r _g _b) (Utilities|Struct|BreakLinearColor _horizoncolor))
  (bind _outactors (Actor|GetAllActorsOfClass "/Engine/EngineSky/BP_Sky_Sphere.BP_Sky_Sphere_C"))
  (Variables|/Engine/EngineSky/BP_Sky_Sphere.BP_Sky_Sphere_C|SetColors%20determined%20by%20sun%20position (Utilities|Array|Get(acopy) _outactors) false)
  (Rendering|Material|SetVectorParameterValue (Variables|/Engine/EngineSky/BP_Sky_Sphere.BP_Sky_Sphere_C|GetSky%20material (Utilities|Array|Get(acopy) _outactors)) "Light direction" (Math|Conversions|ToLinearColor(Vector) (Math|Rotator|GetRotationXVector (Variables|Default|GetSunRotation))) :!class /Script/Engine.MaterialInstanceDynamic)
  (Rendering|Material|SetScalarParameterValue (Variables|/Engine/EngineSky/BP_Sky_Sphere.BP_Sky_Sphere_C|GetSky%20material (Utilities|Array|Get(acopy) _outactors)) "Cloud opacity" (* _cloudopacity 0.07) :!class /Script/Engine.MaterialInstanceDynamic)
  (Rendering|Material|SetScalarParameterValue (Variables|/Engine/EngineSky/BP_Sky_Sphere.BP_Sky_Sphere_C|GetSky%20material (Utilities|Array|Get(acopy) _outactors)) "Horizon Falloff" _horizontfalloff :!class /Script/Engine.MaterialInstanceDynamic)
  (Rendering|Material|SetScalarParameterValue (Variables|/Engine/EngineSky/BP_Sky_Sphere.BP_Sky_Sphere_C|GetSky%20material (Utilities|Array|Get(acopy) _outactors)) "sun brightness" _sunbrightness :!class /Script/Engine.MaterialInstanceDynamic)
  (Variables|Default|SetNewVar_0 _r)
  (Variables|Default|SetNewVar_1 _g)
  (Variables|Default|SetNewVar_2 _b)
  (Rendering|Material|SetVectorParameterValue (Variables|/Engine/EngineSky/BP_Sky_Sphere.BP_Sky_Sphere_C|GetSky%20material (Utilities|Array|Get(acopy) _outactors)) "Zenith color" _zenithcolor :!class /Script/Engine.MaterialInstanceDynamic)
  (Rendering|Material|SetVectorParameterValue (Variables|/Engine/EngineSky/BP_Sky_Sphere.BP_Sky_Sphere_C|GetSky%20material (Utilities|Array|Get(acopy) _outactors)) "Horizon Color" _horizoncolor :!class /Script/Engine.MaterialInstanceDynamic)
  (Rendering|Material|SetVectorParameterValue (Variables|/Engine/EngineSky/BP_Sky_Sphere.BP_Sky_Sphere_C|GetSky%20material (Utilities|Array|Get(acopy) _outactors)) "Cloud color" _cloudcolor :!class /Script/Engine.MaterialInstanceDynamic)
  (Rendering|Material|SetVectorParameterValue (Variables|/Engine/EngineSky/BP_Sky_Sphere.BP_Sky_Sphere_C|GetSky%20material (Utilities|Array|Get(acopy) _outactors)) "Overall Color" _overallskycolor :!class /Script/Engine.MaterialInstanceDynamic))

(fn SetNightDay
  (bind _output_get (Variables|Default|SetSunHeight (.SunPolarAngle (Utilities|Struct|BreakWeatherDescription (Class|DynamicWeather|GetWeatherDescription)))))
  (Variables|Default|SetIsNight (< 9e+01 _output_get)))

(fn UpdateDirectionalLight
  (bind _returnvalue (Class|DynamicWeather|GetWeatherDescription))
  (bind (_sundirectionallightintensity _sundirectionallightcolor _sunindirectlightintensity) (Utilities|Struct|BreakWeatherDescription _returnvalue))
  (bind _outactors (Actor|GetAllActorsOfClass "/Script/Engine.DirectionalLight"))
  (bind _output_get (Variables|Default|SetSunRotation (Math|Conversions|RotationFromXVector (Class|KismetMathLibrary|CreateVectorfromYawPitch (.Yaw (Math|Vector|GetYawPitchfromVector (Math|Vector|GetForwardVector (Transformation|GetActorRotation (Utilities|Array|Get(acopy) _outactors))))) (.Pitch (Math|Vector|GetYawPitchfromVector (Class|DynamicWeather|GetSunDirection))) 1.0))))
  (Transformation|SetActorRotation (Utilities|Array|Get(acopy) _outactors) _output_get)
  (Rendering|Components|Light|SetIntensity (Variables|/Script/Engine.Light|GetLightComponent (Utilities|Array|Get(acopy) _outactors)) (* _sundirectionallightintensity 0.2))
  (Rendering|Components|Light|SetLightColor (Variables|/Script/Engine.Light|GetLightComponent (Utilities|Array|Get(acopy) _outactors)) _sundirectionallightcolor true)
  (Class|LightComponent|SetIndirectLightingIntensity (Variables|/Script/Engine.Light|GetLightComponent (Utilities|Array|Get(acopy) _outactors)) (* _sunindirectlightintensity 0.06)))

(fn SetSkylight
  (bind _returnvalue (Class|DynamicWeather|GetWeatherDescription))
  (bind (_name _sunindirectlightintensity _skylightintensity _skylightcolor) (Utilities|Struct|BreakWeatherDescription _returnvalue))
  (bind _outactors (Actor|GetAllActorsOfClass "/Script/Engine.SkyLight"))
  (Rendering|Components|Light|SetLightColor (Variables|/Script/Engine.SkyLight|GetLightComponent (Utilities|Array|Get(acopy) _outactors (Utilities|Array|LastIndex _outactors))) _skylightcolor)
  (Rendering|Components|Light|SetIntensity (Variables|/Script/Engine.SkyLight|GetLightComponent (Utilities|Array|Get(acopy) _outactors (Utilities|Array|LastIndex _outactors))) (* _skylightintensity 0.2))
  (Class|SkyLightComponent|SetIndirectLightingIntensity (Variables|/Script/Engine.SkyLight|GetLightComponent (Utilities|Array|Get(acopy) _outactors (Utilities|Array|LastIndex _outactors))) (* _sunindirectlightintensity 0.06)))

(fn SetPrecipitations
  (bind _returnvalue (Class|DynamicWeather|GetWeatherDescription))
  (bind (_name _bprecipitation _precipitationtype _precipitationamount _precipitationaccumulation _bwind _windintensity) (Utilities|Struct|BreakWeatherDescription _returnvalue))
  (bind _returnvalue_2 (/ _precipitationaccumulation 1e+02))
  (Rendering|SetVisibility (Variables|Default|GetRainParticleSystem) _bprecipitation false)
  (if _bprecipitation
    (Effects|Components|ParticleSystem|SetFloatParameter (Variables|Default|GetRainParticleSystem) "RainDensity" _precipitationamount)
    (Rendering|Material|SetScalarParameterValue "/Game/Static/GenericMaterials/WetPavement/WetRoadComplexParam.WetRoadComplexParam" "RippleIntensity" (* _precipitationamount 0.01) :!class /Script/Engine.KismetMaterialLibrary)
    (Rendering|Material|SetScalarParameterValue "/Game/Static/GenericMaterials/WetPavement/WetRoadComplexParam.WetRoadComplexParam" "Water Level" _returnvalue_2 :!class /Script/Engine.KismetMaterialLibrary)
    (Rendering|Material|SetScalarParameterValue "/Game/Static/GenericMaterials/WetPavement/WetRoadComplexParam.WetRoadComplexParam" "Humidity" (* (+ _returnvalue_2 0.2) (/ _precipitationaccumulation 1e+01)) :!class /Script/Engine.KismetMaterialLibrary)
    (Rendering|Material|SetScalarParameterValue "/Game/Static/GenericMaterials/WetPavement/WetRoadComplexParam.WetRoadComplexParam" "WindIntensity" (/ _windintensity 1e+02) :!class /Script/Engine.KismetMaterialLibrary)
    (else
      (Effects|Components|ParticleSystem|SetFloatParameter (Variables|Default|GetRainParticleSystem) "RainDensity" 0.0)
      (Rendering|Material|SetScalarParameterValue "/Game/Static/GenericMaterials/WetPavement/WetRoadComplexParam.WetRoadComplexParam" "RippleIntensity" 0.0 :!class /Script/Engine.KismetMaterialLibrary)
      (Rendering|Material|SetScalarParameterValue "/Game/Static/GenericMaterials/WetPavement/WetRoadComplexParam.WetRoadComplexParam" "Water Level" 0.0 :!class /Script/Engine.KismetMaterialLibrary)
      (Rendering|Material|SetScalarParameterValue "/Game/Static/GenericMaterials/WetPavement/WetRoadComplexParam.WetRoadComplexParam" "Humidity" 0.0 :!class /Script/Engine.KismetMaterialLibrary))))

(fn SetArtificialLighting
  (bind _outactors (Actor|GetAllActorsOfClass "/Game/Static/Pole/Prop_CityLamp/ArtificialLight.ArtificialLight_C"))
  (for _array_element _outactors
    (Default|SwitchLight _array_element (Variables|Default|GetIsNight))))

(fn ChangeWeatheratRuntime
  (bind _ascarla_game_instance (Utilities|Casting|CastToCarlaGameInstance (Game|GetGameInstance))
    (:then
      (bind _returnvalue (Class|CarlaGameInstance|GetCARLASettings _ascarla_game_instance))
      (bind _index (|IncrementIndex))
      (bind _returnvalue_2 (Class|CarlaSettings|GetWeatherDescriptionbyIndex _returnvalue _index))
      (Development|PrintString (Utilities|String|Append "Changed weather to " (.Name (Utilities|Struct|BreakWeatherDescription _returnvalue_2))) false)
      (Class|DynamicWeather|ActivateWeatherDescription _returnvalue_2)
      (return (> (.PrecipitationAmount (Utilities|Struct|BreakWeatherDescription _returnvalue_2)) 1e+01)))
    (:CastFailed
      (Development|PrintString "Game instance is not a Carla game instance!" false))))