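; Construction-script spline mesh repeater that builds a deformed static mesh segment between each pair of neighboring spline points.
; Segments follow the local point tangents, with configurable forward axis and collision, and GapDistance insets their ends along local X only rather than along the spline.
; A valid Material feeds a dynamic material instance that receives top wall, details and main color parameters.
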(event EventBeginPlay)

(event Collision|EventActorBeginOverlap
  (params (OtherActor :type Actor%20Object%20Reference)))

(event EventTick
  (params (DeltaSeconds :type Float%20%28single-precision%29)))

(fn ConstructionScript
  (bind _spline (Variables|Default|GetSpline))
  (bind _gapdistance (Variables|Default|GetGapDistance))
  (bind _material (Variables|Default|GetMaterial))
  (for _index (range 0 (- (Spline|GetNumberOfSplinePoints _spline) 2))
    (bind _returnvalue (AddComponent|AddSplineMeshComponent false))
    (Components|StaticMesh|SetStaticMesh _returnvalue (Variables|Default|GetstaticMesh))
    (SplineMesh|SetForwardAxis _returnvalue (Variables|Default|Getforward%20axis) true)
    (Transformation|AttachComponentToComponent _returnvalue _spline "None" "KeepRelative" "KeepRelative" "KeepRelative" true)
    (SplineMesh|SetStartandEnd _returnvalue (Math|Vector|MakeVector (+ (.X (Math|Vector|BreakVector (.Location (Spline|GetLocationandTangentatSplinePoint _spline _index "Local")))) _gapdistance) (.Y (Math|Vector|BreakVector (.Location (Spline|GetLocationandTangentatSplinePoint _spline _index "Local")))) (.Z (Math|Vector|BreakVector (.Location (Spline|GetLocationandTangentatSplinePoint _spline _index "Local"))))) (.Tangent (Spline|GetLocationandTangentatSplinePoint _spline _index "Local")) (Math|Vector|MakeVector (- (.X (Math|Vector|BreakVector (.Location (Spline|GetLocationandTangentatSplinePoint _spline (+ _index 1) "Local")))) _gapdistance) (.Y (Math|Vector|BreakVector (.Location (Spline|GetLocationandTangentatSplinePoint _spline (+ _index 1) "Local")))) (.Z (Math|Vector|BreakVector (.Location (Spline|GetLocationandTangentatSplinePoint _spline (+ _index 1) "Local"))))) (.Tangent (Spline|GetLocationandTangentatSplinePoint _spline (+ _index 1) "Local")) true :!class /Script/Engine.SplineMeshComponent)
    (Collision|SetCollisionEnabled _returnvalue (Variables|Default|GetColission%20enabled)))
  (if (Utilities|IsValid _material)
    (Rendering|Material|SetMaterial _returnvalue 0 _material)
    (bind _returnvalue_2 (Rendering|Material|CreateDynamicMaterialInstance _returnvalue 0 _material :!class /Script/Engine.PrimitiveComponent))
    (Rendering|Material|SetVectorParameterValue _returnvalue_2 "TopWallColor" (Variables|Default|GetTopWallColor) :!class /Script/Engine.MaterialInstanceDynamic)
    (Rendering|Material|SetVectorParameterValue _returnvalue_2 "DetailsColor" (Variables|Default|GetDetailsColor) :!class /Script/Engine.MaterialInstanceDynamic)
    (Rendering|Material|SetVectorParameterValue _returnvalue_2 "MainMaterialColor" (Variables|Default|GetMainMaterialColor) :!class /Script/Engine.MaterialInstanceDynamic)
    (else
      (SplineMesh|SetForwardAxis _returnvalue (Variables|Default|Getforward%20axis) true)
      (Transformation|AttachComponentToComponent _returnvalue _spline "None" "KeepRelative" "KeepRelative" "KeepRelative" true)
      (SplineMesh|SetStartandEnd _returnvalue (Math|Vector|MakeVector (+ (.X (Math|Vector|BreakVector (.Location (Spline|GetLocationandTangentatSplinePoint _spline _index "Local")))) _gapdistance) (.Y (Math|Vector|BreakVector (.Location (Spline|GetLocationandTangentatSplinePoint _spline _index "Local")))) (.Z (Math|Vector|BreakVector (.Location (Spline|GetLocationandTangentatSplinePoint _spline _index "Local"))))) (.Tangent (Spline|GetLocationandTangentatSplinePoint _spline _index "Local")) (Math|Vector|MakeVector (- (.X (Math|Vector|BreakVector (.Location (Spline|GetLocationandTangentatSplinePoint _spline (+ _index 1) "Local")))) _gapdistance) (.Y (Math|Vector|BreakVector (.Location (Spline|GetLocationandTangentatSplinePoint _spline (+ _index 1) "Local")))) (.Z (Math|Vector|BreakVector (.Location (Spline|GetLocationandTangentatSplinePoint _spline (+ _index 1) "Local"))))) (.Tangent (Spline|GetLocationandTangentatSplinePoint _spline (+ _index 1) "Local")) true :!class /Script/Engine.SplineMeshComponent)
      (Collision|SetCollisionEnabled _returnvalue (Variables|Default|GetColission%20enabled)))))