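; Vehicle spawner Blueprint that creates a vehicle from its VehicleModels list at a supplied transform when SpawnVehicle is called.
; GetNextVehicle cycles through the list round-robin with an incrementing index and modulo wrap.
; The spawn is skipped if the list is empty or the location is colliding, and each new vehicle receives a random engine.
; A random-pick alternative, GetRandomVehicle, exists but is not used by SpawnVehicle, and the event graph is empty.
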(event EventBeginPlay)

(event Collision|EventActorBeginOverlap
  (params (OtherActor :type Actor%20Object%20Reference)))

(event EventTick
  (params (DeltaSeconds :type Float%20%28single-precision%29)))

(fn ConstructionScript)

(fn SpawnVehicle
  (params (SpawnTransform :type Transform%20%28by%20ref%29))
  (bind _vehiclemodels (Variables|VehicleSpawner|GetVehicleModels))
  (if (> (Utilities|Array|Length _vehiclemodels) 0)
    (bind _vehiclemodel (Utilities|GetNextVehicle _vehiclemodels))
    (bind _returnvalue (Class|ActorwithRandomEngine|GetRandomEngine))
    (bind _returnvalue_2 (Game|SpawnActorfromClass _vehiclemodel SpawnTransform "DontSpawnIfColliding" 0 _returnvalue 0))
    (return _returnvalue_2)
    (else
      (return 0))))