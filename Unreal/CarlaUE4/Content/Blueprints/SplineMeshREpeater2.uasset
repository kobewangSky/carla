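; Spline mesh repeater that builds a segmented piece, apparently a wall, along a spline in its Construction Script.
; OpeningMesh spans the first segment, BodyMesh repeats over the following segments, and ClosingMesh runs back to point 0 to close the loop.
; Duplicated collapsed graphs create each spline mesh with a forward axis and a dynamic material carrying three colour parameters.
; A DisableCollision flag toggles collision on the pieces; the event graph is empty.
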(event EventBeginPlay)

(event Collision|EventActorBeginOverlap
  (params (OtherActor :type Actor%20Object%20Reference)))

(event EventTick
  (params (DeltaSeconds :type Float%20%28single-precision%29)))

(fn ConstructionScript
  (bind _spline (Variables|Default|GetSpline))
  (bind (_location _tangent) (Spline|GetLocationandTangentatSplinePoint _spline 1 "Local"))
  (bind (_location_2 _tangent_2) (Spline|GetLocationandTangentatSplinePoint _spline 0 "Local"))
  (bind (_location_3 _tangent_3) (Spline|GetLocationandTangentatSplinePoint _spline 0 "Local"))
  (bind _returnvalue (|CollapseGraph_2_3 (Variables|Default|GetOpeningMesh)))
  (Transformation|AttachComponentToComponent _returnvalue _spline "None" "KeepRelative" "KeepRelative" "KeepRelative" true)
  (SplineMesh|SetStartandEnd _returnvalue _location_3 _tangent_3 _location _tangent true :!class /Script/Engine.SplineMeshComponent)
  (for _index (range 1 (- (Spline|GetNumberOfSplinePoints _spline) 2))
    (bind _returnvalue_2 (|CollapseGraph_2 (Variables|Default|GetBodyMesh)))
    (Transformation|AttachComponentToComponent _returnvalue_2 _spline "None" "KeepRelative" "KeepRelative" "KeepRelative" true)
    (SplineMesh|SetStartandEnd _returnvalue_2 (.ReturnValue (|CollapseGraph_0 (.Location (Spline|GetLocationandTangentatSplinePoint _spline _index "Local")) (.Location (Spline|GetLocationandTangentatSplinePoint _spline (+ _index 1) "Local")))) (.Tangent (Spline|GetLocationandTangentatSplinePoint _spline _index "Local")) (.ReturnValue2 (|CollapseGraph_0 (.Location (Spline|GetLocationandTangentatSplinePoint _spline _index "Local")) (.Location (Spline|GetLocationandTangentatSplinePoint _spline (+ _index 1) "Local")))) (.Tangent (Spline|GetLocationandTangentatSplinePoint _spline (+ _index 1) "Local")) true :!class /Script/Engine.SplineMeshComponent)
    (Collision|SetCollisionEnabled _returnvalue_2 (select (Variables|Default|GetDisableCollision) "NoCollision" "QueryAndPhysics")))
  (bind _returnvalue_3 (|CollapseGraph_2_2 (Variables|Default|GetClosingMesh)))
  (Transformation|AttachComponentToComponent _returnvalue_3 _spline "None" "KeepRelative" "KeepRelative" "KeepRelative" true)
  (SplineMesh|SetStartandEnd _returnvalue_3 (.Location (Spline|GetLocationandTangentatSplinePoint _spline _index "Local")) (.Tangent (Spline|GetLocationandTangentatSplinePoint _spline _index "Local")) _location_2 _tangent_2 true :!class /Script/Engine.SplineMeshComponent)
  (Collision|SetCollisionEnabled _returnvalue_2 (select (Variables|Default|GetDisableCollision) "NoCollision" "QueryAndPhysics")))