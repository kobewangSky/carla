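; Construction-script actor that repeats a static mesh along an editable spline, bending one spline mesh component across each segment between neighboring points.
; Each piece takes its endpoints and tangents from the spline in local space, with a configurable gap offset applied only on the X axis.
; Forward axis and collision are configurable, and an optional dynamic material instance applies top wall, details and main color parameters to the first material slot.
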(event EventBeginPlay)

(event Collision|EventActorBeginOverlap
  (params (OtherActor :type Actor%20Object%20Reference)))

(event EventTick
  (params (DeltaSeconds :type Float%20%28single-precision%29)))

(fn ConstructionScript
  (bind _spline (Variables|Default|GetSpline))
  (bind _gapdistance (Variables|Default|GetGapDistance))
  (bind _material (Variables|Default|GetMaterial))
  (if (Utilities|IsValid _material)
    (bind _returnvalue (Rendering|Material|CreateDynamicMaterialInstance _material :!class /Script/Engine.KismetMaterialLibrary))
    (bind _output_get (Variables|Default|SetDynamicMaterial _returnvalue))
    (Rendering|Material|SetVectorParameterValue _output_get "TopWallColor" (Variables|Default|GetTopWallColor) :!class /Script/Engine.MaterialInstanceDynamic)
    (Rendering|Material|SetVectorParameterValue _output_get "DetailsColor" (Variables|Default|GetDetailsColor) :!class /Script/Engine.MaterialInstanceDynamic)
    (Rendering|Material|SetVectorParameterValue _output_get "MainMaterialColor" (Variables|Default|GetMainMaterialColor) :!class /Script/Engine.MaterialInstanceDynamic))
  (for _index (range 0 (- (Spline|GetNumberOfSplinePoints _spline) 2))
    (bind _returnvalue_2 (AddComponent|AddSplineMeshComponent false))
    (Components|StaticMesh|SetStaticMesh _returnvalue_2 (Variables|Default|GetstaticMesh))
    (Utilities|IsValid (Variables|Default|GetDynamicMaterial)
      (:Is%20Valid
        (Rendering|Material|SetMaterial _returnvalue_2 0 (Variables|Default|GetDynamicMaterial)))
      (:Is%20Not%20Valid
        _))
    (SplineMesh|SetForwardAxis _returnvalue_2 (Variables|Default|Getforward%20axis) true)
    (Transformation|AttachComponentToComponent _returnvalue_2 _spline "None" "KeepRelative" "KeepRelative" "KeepRelative" true)
    (SplineMesh|SetStartandEnd _returnvalue_2 (Math|Vector|MakeVector (+ (.X (Math|Vector|BreakVector (.Location (Spline|GetLocationandTangentatSplinePoint _spline _index "Local")))) _gapdistance) (.Y (Math|Vector|BreakVector (.Location (Spline|GetLocationandTangentatSplinePoint _spline _index "Local")))) (.Z (Math|Vector|BreakVector (.Location (Spline|GetLocationandTangentatSplinePoint _spline _index "Local"))))) (.Tangent (Spline|GetLocationandTangentatSplinePoint _spline _index "Local")) (Math|Vector|MakeVector (- (.X (Math|Vector|BreakVector (.Location (Spline|GetLocationandTangentatSplinePoint _spline (+ _index 1) "Local")))) _gapdistance) (.Y (Math|Vector|BreakVector (.Location (Spline|GetLocationandTangentatSplinePoint _spline (+ _index 1) "Local")))) (.Z (Math|Vector|BreakVector (.Location (Spline|GetLocationandTangentatSplinePoint _spline (+ _index 1) "Local"))))) (.Tangent (Spline|GetLocationandTangentatSplinePoint _spline (+ _index 1) "Local")) true :!class /Script/Engine.SplineMeshComponent)
    (Collision|SetCollisionEnabled _returnvalue_2 (Variables|Default|GetColission%20enabled))))