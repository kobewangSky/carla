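; Climate preset Blueprint that sets the level's lighting and sky to a noon look from its Construction Script.
; Helper functions find the first DirectionalLight, BP_Sky_Sphere and SkyLight in the level and overwrite their sun angle, intensity, color and cloud settings.
; It also zeroes "Min water" in the WetRoadComplexParam material parameter collection.
; The PostProcessVolume lookup is unused, Changesunposition is empty and NewFunction_0 is an uncalled directional-light variant.
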(event EventBeginPlay)

(event Collision|EventActorBeginOverlap
  (params (OtherActor :type Actor%20Object%20Reference)))

(event EventTick
  (params (DeltaSeconds :type Float%20%28single-precision%29)))

(fn ConstructionScript
  (CallFunction|DirectionalLightChanges)
  (CallFunction|SkySphereChanges)
  (CallFunction|SkyLightChanges)
  (Rendering|Material|SetScalarParameterValue "/Game/Static/GenericMaterials/WetPavement/WetRoadComplexParam.WetRoadComplexParam" "Min water" 0.0 :!class /Script/Engine.KismetMaterialLibrary)
  (Actor|GetAllActorsOfClass "/Script/Engine.PostProcessVolume"))

(fn Changesunposition
  (params (Position :type Vector%202D%20Structure)))

(fn NewFunction0
  (bind _outactors (Actor|GetAllActorsOfClass "/Script/Engine.DirectionalLight"))
  (Transformation|SetActorRotation (Utilities|Array|Get(acopy) _outactors) "-47.000000,-170.000000,166.000000")
  (Rendering|Components|Light|SetIntensity (Variables|/Script/Engine.Light|GetLightComponent (Utilities|Array|Get(acopy) _outactors)) 5.0)
  (Rendering|Components|Light|SetLightColor (Variables|/Script/Engine.Light|GetLightComponent (Utilities|Array|Get(acopy) _outactors)) "(R=255.000000,G=239.000000,B=194.000000,A=1.000000)" false)
  (Class|LightComponent|SetIndirectLightingIntensity (Variables|/Script/Engine.Light|GetLightComponent (Utilities|Array|Get(acopy) _outactors)) 1.0)
  (Class|LightComponent|SetEnableLightShaftBloom (Variables|/Script/Engine.Light|GetLightComponent (Utilities|Array|Get(acopy) _outactors)) true))

(fn DirectionalLightChanges
  (bind _outactors (Actor|GetAllActorsOfClass "/Script/Engine.DirectionalLight"))
  (Transformation|SetActorRotation (Utilities|Array|Get(acopy) _outactors) "-47.000000,-170.000000,166.000000")
  (Rendering|Components|Light|SetIntensity (Variables|/Script/Engine.Light|GetLightComponent (Utilities|Array|Get(acopy) _outactors)) 5.0)
  (Rendering|Components|Light|SetLightColor (Variables|/Script/Engine.Light|GetLightComponent (Utilities|Array|Get(acopy) _outactors)) "(R=1.000000,G=0.937000,B=0.761000,A=1.000000)" false)
  (Class|LightComponent|SetIndirectLightingIntensity (Variables|/Script/Engine.Light|GetLightComponent (Utilities|Array|Get(acopy) _outactors)) 1.0)
  (Class|LightComponent|SetEnableLightShaftBloom (Variables|/Script/Engine.Light|GetLightComponent (Utilities|Array|Get(acopy) _outactors)) true))

(fn SkySphereChanges
  (bind _outactors (Actor|GetAllActorsOfClass "/Engine/EngineSky/BP_Sky_Sphere.BP_Sky_Sphere_C"))
  (Variables|/Engine/EngineSky/BP_Sky_Sphere.BP_Sky_Sphere_C|SetColors%20determined%20by%20sun%20position (Utilities|Array|Get(acopy) _outactors) true)
  (Variables|/Engine/EngineSky/BP_Sky_Sphere.BP_Sky_Sphere_C|SetSun%20brightness (Utilities|Array|Get(acopy) _outactors) 5e+01)
  (Variables|/Engine/EngineSky/BP_Sky_Sphere.BP_Sky_Sphere_C|SetCloud%20opacity (Utilities|Array|Get(acopy) _outactors) 0.7)
  (Variables|/Engine/EngineSky/BP_Sky_Sphere.BP_Sky_Sphere_C|SetSun%20height (Utilities|Array|Get(acopy) _outactors) 0.528341)
  (Variables|/Engine/EngineSky/BP_Sky_Sphere.BP_Sky_Sphere_C|SetHorizon%20Falloff (Utilities|Array|Get(acopy) _outactors) 3.0)
  (Variables|/Engine/EngineSky/BP_Sky_Sphere.BP_Sky_Sphere_C|SetZenith%20Color (Utilities|Array|Get(acopy) _outactors) "(R=0.033989,G=0.109000,B=0.295000,A=1.000000)")
  (Variables|/Engine/EngineSky/BP_Sky_Sphere.BP_Sky_Sphere_C|SetHorizon%20color (Utilities|Array|Get(acopy) _outactors) "(R=1.979000,G=2.580000,B=3.000000,A=1.000000)")
  (Variables|/Engine/EngineSky/BP_Sky_Sphere.BP_Sky_Sphere_C|SetCloud%20color (Utilities|Array|Get(acopy) _outactors) "(R=0.855000,G=0.919020,B=1.000000,A=1.000000)")
  (Variables|/Engine/EngineSky/BP_Sky_Sphere.BP_Sky_Sphere_C|SetOverall%20Color (Utilities|Array|Get(acopy) _outactors) "(R=1.000000,G=1.000000,B=1.000000,A=1.000000)"))

(fn SkyLightChanges
  (bind _outactors (Actor|GetAllActorsOfClass "/Script/Engine.SkyLight"))
  (Rendering|Components|Light|SetIntensity (Variables|/Script/Engine.SkyLight|GetLightComponent (Utilities|Array|Get(acopy) _outactors)) 1.5)
  (Rendering|Components|Light|SetLightColor (Variables|/Script/Engine.SkyLight|GetLightComponent (Utilities|Array|Get(acopy) _outactors)) "(R=0.541000,G=0.514000,B=0.392000,A=1.000000)")
  (Class|SkyLightComponent|SetIndirectLightingIntensity (Variables|/Script/Engine.SkyLight|GetLightComponent (Utilities|Array|Get(acopy) _outactors)) 6.0))