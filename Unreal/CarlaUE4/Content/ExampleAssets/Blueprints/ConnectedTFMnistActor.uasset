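; Example actor that tests MNIST digit prediction through a Python TensorFlow component, using preset textures or drawings received over Socket.IO.
; Number keys choose a test image and F sends it; incoming strokes are rasterized to a texture and sent automatically.
; Returned JSON updates the result sprite and prediction text.
; G toggles training, whose events update accuracy text and spawn sprite actors from pixel data.
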(event OnEvent(TensorflowComponent)
  (params (Event :type String) (Data :type String))
  (Utilities|FlowControl|Sequence
    (:then_0
      (if (Utilities|Enum|Equal(Enum) Event "PixelEvent")
        (CallFunction|OnPixelEvent Data)))
    (:then_1
      (if (Utilities|Enum|Equal(Enum) Event "TrainingUpdateEvent")
        (CallFunction|OnTrainingUpdateEvent Data)))))

(event OnInputResults(TensorflowComponent)
  (params (Results :type String))
  (bind _returnvalue (Class|SIOJsonValue|ValuefromJsonString Results))
  (bind _resultdata (Variables|Default|GetResultData))
  (bind (_pixels _size) (Utilities|Struct|BreakImageStruct _resultdata))
  (bind _returnvalue_2 (Class|SIOJLibrary|ToJsonObject(JsonValue) _returnvalue))
  (bind _returnvalue_3 (Class|SIOJsonObject|GetNumberField _returnvalue_2 "prediction"))
  (bind _returnvalue_4 (Math|Float|Truncate _returnvalue_3))
  (bind _returnvalue_5 (Utilities|String|ToString(Integer) _returnvalue_4))
  (bind _returnvalue_6 (Utilities|String|Append "Prediction: " _returnvalue_5))
  (Class|SIOJLibrary|JsonObjecttoStruct _returnvalue_2 _resultdata) ; we know this is compatible with an ImageStruct format so convert it to a ue4 struct
  (CallFunction|SetResultTexture (Class|TensorFlowBlueprintLibrary|ToTexture2D(GrayScaleFloatArray) _pixels _size))
  (Development|PrintString _returnvalue_6)
  (Rendering|Components|TextRender|SetText (Variables|Default|GetPredictionText) (Utilities|Text|ToText(String) _returnvalue_6)))

(event OnTrainingComplete(TensorflowComponent)
  (params (SummaryJson :type String))
  (bind _returnvalue (Class|SIOJsonValue|AsObject (Class|SIOJsonValue|ValuefromJsonString SummaryJson)))
  (Development|PrintString (Utilities|String|Append "Training complete in: " (Utilities|String|ToString(Float) (Class|SIOJsonObject|GetNumberField _returnvalue "elapsed"))))
  (Rendering|Components|TextRender|SetText (Variables|Default|GetPredictionText) (Utilities|Text|ToText(String) (Utilities|String|Append "Training complete in: " (Utilities|String|ToString(Float) (Class|SIOJsonObject|GetNumberField _returnvalue "elapsed"))))))

(event EventBeginPlay
  (CallFunction|BindSocketioEvents)
  (CallFunction|UpdateSendTexture))

(event Input|KeyboardEvents|F
  (params (Key :type Key%20Structure))
  (:Pressed
    (Default|SendJsonInputTexture (Variables|Default|GetTensorflowComponent) (Variables|Default|GetExampleTexture) false true)))

(event Input|KeyboardEvents|G
  (params (Key :type Key%20Structure))
  (:Pressed
    (Utilities|FlowControl|FlipFlop
      (:A
        (Default|StopTraining (Variables|Default|GetTensorflowComponent)))
      (:B
        (Default|BeginTraining (Variables|Default|GetTensorflowComponent))))))

(event Input|KeyboardEvents|2
  (params (Key :type Key%20Structure))
  ;[1 1 1] 0-9
  (:Pressed
    (Variables|Default|SetExampleTexture "/Game/ExampleAssets/Materials/test2.test2")
    (Development|PrintString "changed to 2")
    (CallFunction|UpdateSendTexture)))

(event Input|KeyboardEvents|H
  (params (Key :type Key%20Structure))
  (:Pressed
    (Default|Clear (Variables|Default|GetStrokeTextureComponent) "(R=1.000000,G=1.000000,B=1.000000,A=1.000000)")))

(event Input|KeyboardEvents|3
  (params (Key :type Key%20Structure))
  ;[1 1 1] 0-9
  (:Pressed
    (Variables|Default|SetExampleTexture "/Game/ExampleAssets/Materials/test3.test3")
    (Development|PrintString "changed to 3")
    (CallFunction|UpdateSendTexture)))

(event Input|KeyboardEvents|1
  (params (Key :type Key%20Structure))
  ;[1 1 1] 0-9
  (:Pressed
    (Variables|Default|SetExampleTexture "/Game/ExampleAssets/Materials/test1.test1")
    (Development|PrintString "changed to 1")
    (CallFunction|UpdateSendTexture)))

(event Input|KeyboardEvents|0
  (params (Key :type Key%20Structure))
  ;[1 1 1] 0-9
  (:Pressed
    (Variables|Default|SetExampleTexture "/Game/ExampleAssets/Materials/test0.test0")
    (Development|PrintString "changed to 0")
    (CallFunction|UpdateSendTexture)))

(event Input|KeyboardEvents|4
  (params (Key :type Key%20Structure))
  ;[1 1 1] 0-9
  (:Pressed
    (Variables|Default|SetExampleTexture "/Game/ExampleAssets/Materials/test4.test4")
    (Development|PrintString "changed to 4")
    (CallFunction|UpdateSendTexture)))

(event Input|KeyboardEvents|5
  (params (Key :type Key%20Structure))
  ;[1 1 1] 0-9
  (:Pressed
    (Variables|Default|SetExampleTexture "/Game/ExampleAssets/Materials/test5.test5")
    (Development|PrintString "changed to 5")
    (CallFunction|UpdateSendTexture)))

(event Input|KeyboardEvents|6
  (params (Key :type Key%20Structure))
  ;[1 1 1] 0-9
  (:Pressed
    (Variables|Default|SetExampleTexture "/Game/ExampleAssets/Materials/test6.test6")
    (Development|PrintString "changed to 6")
    (CallFunction|UpdateSendTexture)))

(event Input|KeyboardEvents|7
  (params (Key :type Key%20Structure))
  ;[1 1 1] 0-9
  (:Pressed
    (Variables|Default|SetExampleTexture "/Game/ExampleAssets/Materials/test7.test7")
    (Development|PrintString "changed to 7")
    (CallFunction|UpdateSendTexture)))

(event Input|KeyboardEvents|8
  (params (Key :type Key%20Structure))
  ;[1 1 1] 0-9
  (:Pressed
    (Variables|Default|SetExampleTexture "/Game/ExampleAssets/Materials/test8.test8")
    (Development|PrintString "changed to 8")
    (CallFunction|UpdateSendTexture)))

(event Input|KeyboardEvents|9
  (params (Key :type Key%20Structure))
  ;[1 1 1] 0-9
  (:Pressed
    (Variables|Default|SetExampleTexture "/Game/ExampleAssets/Materials/test9.test9")
    (Development|PrintString "changed to 9")
    (CallFunction|UpdateSendTexture)))

(event OnConnected(SocketIOClient)
  (params (SessionId :type String) (bIsReconnection :type Boolean))
  (Class|SocketIOClientComponent|Emit (Variables|Default|GetSocketIOClient) "ue4client" (Class|SIOJLibrary|ToJsonValue(String) (Utilities|String|MakeLiteralString)) "/"))

(fn ConstructionScript
  (Variables|/TensorFlow/TensorflowComponent.TensorflowComponent_C|SetTensorFlowModule (Variables|Default|GetTensorflowComponent) (Variables|Default|GetPythonTFModule))
  (Variables|/TensorFlow/TensorflowComponent.TensorflowComponent_C|SetShouldRetrain (Variables|Default|GetTensorflowComponent) (Variables|Default|GetForceRetrain)))

(fn SetResultTexture
  (params (Texture :type Texture%202D%20Object%20Reference))
  (bind _output_get (Variables|Default|SetResultTexture Texture))
  (Rendering|Components|Sprite|SetSprite (Variables|Default|GetReceive) _output_get))

(fn BindSocketioEvents
  (Class|SocketIOClientComponent|BindEventtoFunction (Variables|Default|GetSocketIOClient) "drawing" "OnDrawing" 0 "/"))

(fn OnDrawing
  (params (Message :type SIO%20Json%20Value%20Object%20Reference))
  (bind _drawing (Variables|Default|GetDrawing))
  (Development|PrintString "received drawing")
  (Class|SIOJLibrary|JsonObjecttoStruct (Class|SIOJLibrary|ToJsonObject(JsonValue) Message) _drawing) ; convert to drawing struct
  (bind _texture (CallFunction|DrawingtoTexture _drawing)) ; convert our strokes to a texture
  (Default|SendJsonInputTexture (Variables|Default|GetTensorflowComponent) _texture false true))

(fn DrawingtoTexture
  (params (DrawingStruct :type Drawing%20Struct%20Structure))
  (Default|Clear (Variables|Default|GetStrokeTextureComponent) "(R=1.000000,G=1.000000,B=1.000000,A=1.000000)")
  (for _array_element (Utilities|Struct|BreakDrawingStruct DrawingStruct) ; for all strokes
    (LocalVariables|SetPrevious (Utilities|Array|Get(acopy) (Utilities|Struct|BreakStrokeStruct _array_element)))
    (for _array_element_2 (Utilities|Struct|BreakStrokeStruct _array_element) ; for each stroke
      (Default|DrawLine (Variables|Default|GetStrokeTextureComponent) (LocalVariables|GetPrevious) _array_element_2 "(R=0.000000,G=0.000000,B=0.000000,A=1.000000)" (Variables|Default|GetStrokeThickness))
      (LocalVariables|SetPrevious _array_element_2)))
  (bind _texture (Default|GetTexture (Variables|Default|GetStrokeTextureComponent)))
  (return _texture))

(fn UpdateSendTexture
  (Rendering|Components|Sprite|SetSprite (Variables|Default|GetSend) (Variables|Default|GetExampleTexture)))

(fn SpawnTextureatSpawn
  (params (Texture :type Texture%202D%20Object%20Reference) (SpawnLocation :type Actor%20Object%20Reference) (Spread :type Float%20%28single-precision%29))
  (bind _returnvalue (Game|SpawnActorfromClass "/Game/ExampleAssets/Blueprints/SpriteActor.SpriteActor_C" (Math|Transform|MakeTransform (+ (Transformation|GetActorLocation SpawnLocation) (* (Math|Random|RandomUnitVector) Spread)) "0, 0, 0" "1,1,1") "Undefined" 0 0))
  (Default|SetTexture _returnvalue Texture))

(fn OnPixelEvent
  (params (PixelJson :type String))
  (bind _pixeleventdata (LocalVariables|GetPixelEventData))
  (bind (_pixels _size) (Utilities|Struct|BreakImageStruct _pixeleventdata))
  (Class|SIOJLibrary|JsonObjecttoStruct (Class|SIOJLibrary|ToJsonObject(JsonValue) (Class|SIOJsonValue|ValuefromJsonString PixelJson)) _pixeleventdata)
  (CallFunction|SpawnTextureatSpawn (Class|TensorFlowBlueprintLibrary|ToTexture2D(GrayScaleFloatArray) _pixels _size) (Variables|Default|GetSpawnLocation) 5e+01))

(fn OnTrainingUpdateEvent
  (params (PixelJson :type String))
  (Class|SIOJLibrary|JsonObjecttoStruct (Class|SIOJLibrary|ToJsonObject(JsonValue) (Class|SIOJsonValue|ValuefromJsonString PixelJson)) (LocalVariables|GetCallbackLog))
  (Rendering|Components|TextRender|SetText (Variables|Default|GetPredictionText) (Utilities|Text|ToText(String) (Utilities|String|Append "Training acc: " (Utilities|String|ToString(Float) (.acc (LocalVariables|GetCallbackLog)))))))